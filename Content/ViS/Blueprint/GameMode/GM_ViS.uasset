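; GM_ViS is a game mode that overrides ReadyToEndMatch to decide when the match ends.
; It loops over the player array, casting each entry to PS_Player, and returns false at the first player failing the test.
; The match ends only if every player is on one specific team, controls a CHAR_Voleur (thief) and is outside one particular VoleurState.
; Debug prints show player count and match end.
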(event `self.ReceiveBeginPlay`)

(fn `ReadyToEndMatch`
  (returns (ReturnValue :type Boolean))
  (bind _playerarray (`GameStateBase.PlayerArray` (`GameplayStatics.GetGameState`)))
  (`KismetSystemLibrary.PrintString` (`KismetStringLibrary.Conv_IntToString` (`KismetArrayLibrary.Array_Length` _playerarray)))
  (for _array_element _playerarray
    (bind _asps_player (cast `/Game/ViS/Blueprint/Player/PS_Player` _array_element))
    (bind (_aschar_voleur _bsuccess) (cast `/Game/ViS/Blueprint/Character/CHAR_Voleur` (`Controller.K2_GetPawn` (`PlayerState.GetPlayerController` _asps_player)) :!pure true))
    (if (not (and (`|EnumEquality` (`/Game/ViS/Blueprint/Player/PS_Player.Team` _asps_player) "NewEnumerator1") _bsuccess (`|EnumInequality` (`/Game/ViS/Blueprint/Character/CHAR_Voleur.VoleurState` _aschar_voleur) "NewEnumerator2")))
      (return false)))
  (`KismetSystemLibrary.PrintString` "GM END")
  (return true))

(fn `UserConstructionScript`)