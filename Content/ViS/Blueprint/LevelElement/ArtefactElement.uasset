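; Capturable artefact actor that thieves steal by standing in its overlap area, registering itself with GS_ViS in the construction script.
; A timeline drives capture progress, speeding up with the count of inside thieves, freezing while guards contest, and reversing once all thieves leave.
; Completion hides the mesh and credits the artefact to the last thief to enter through PS_Player.
; Overlapping characters show or hide the capture state display.
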(event `self.ReceiveActorBeginOverlap`
  (params (OtherActor :type "Actor Object Reference"))
  ;[1 1 1] Capture with thief
  (bind _aschar_main (cast `/Game/ViS/Blueprint/Character/CHAR_Main` OtherActor))
  (`/Game/ViS/Blueprint/Character/CHAR_Main.DisplayArtefactCaptureState` _aschar_main self)
  (bind _aschar_voleur (cast `/Game/ViS/Blueprint/Character/CHAR_Voleur` OtherActor)
    (:`then`
      (if (`/Game/ViS/Blueprint/Character/CHAR_Voleur.IsInside` _aschar_voleur)
        (`/Engine/EditorBlueprintResources/StandardMacros.IncrementInt` (`self.NbVoleur`)
          (:`  `
            (set `self.LatestCapturingPlayer` _aschar_voleur)
            (if (not (`self.IsStolen`))
              (`self.UpdateCaptureRate`)
              (bind (_direction _capturepercentage) (`Timeline|CaptureTimeline` :!label _label)
                (:`Update`
                  (set `self.CapturePercentage` _capturepercentage))
                (:`Finished`
                  (bind _output_get (set `self.IsStolen` (>= (`self.CapturePercentage`) 1.0)))
                  (if _output_get
                    (`SceneComponent.SetVisibility` (`self.StaticMesh`) false false)
                    (bind _asps_player (cast `/Game/ViS/Blueprint/Player/PS_Player` (`Pawn.PlayerState` (`self.LatestCapturingPlayer`))))
                    (`KismetArrayLibrary.Array_Add` (`/Game/ViS/Blueprint/Player/PS_Player.CapturedArtefacts` _asps_player) self)))))))))
    (:`CastFailed`
      (cast `/Game/ViS/Blueprint/Character/CHAR_Garde` OtherActor)
      (`/Engine/EditorBlueprintResources/StandardMacros.IncrementInt` (`self.NbGarde`)
        (:`  `
          (`self.UpdateCaptureRate`))))))

(event `self.ReceiveActorEndOverlap`
  (params (OtherActor :type "Actor Object Reference"))
  ;[1 1 1] Capture with thief
  (bind _aschar_main (cast `/Game/ViS/Blueprint/Character/CHAR_Main` OtherActor))
  (`/Game/ViS/Blueprint/Character/CHAR_Main.HideArtefactCaptureState` _aschar_main self)
  (bind _aschar_voleur (cast `/Game/ViS/Blueprint/Character/CHAR_Voleur` OtherActor)
    (:`then`
      (if (`/Game/ViS/Blueprint/Character/CHAR_Voleur.IsInside` _aschar_voleur)
        (`/Engine/EditorBlueprintResources/StandardMacros.DecrementInt` (`self.NbVoleur`)
          (:`  `
            (`self.UpdateCaptureRate`)
            (if (and (<= (`self.NbVoleur`) 0) (not (`self.IsStolen`)))
              (goto _label :!via `Reverse`))))))
    (:`CastFailed`
      (cast `/Game/ViS/Blueprint/Character/CHAR_Garde` OtherActor)
      (`/Engine/EditorBlueprintResources/StandardMacros.DecrementInt` (`self.NbGarde`)
        (:`  `
          (`self.UpdateCaptureRate`))))))

(fn `UpdateCaptureRate`
  (`TimelineComponent.SetPlayRate` (`self.CaptureTimeLine`) (`KismetMathLibrary.SelectFloat` 1.0 (`KismetMathLibrary.SelectFloat` 0.0 (`KismetMathLibrary.Conv_IntToDouble` (`self.NbVoleur`)) (> (`self.NbGarde`) 0)) (<= (`self.NbVoleur`) 0))))

(fn `UserConstructionScript`
  (bind _asgs_vi_s (cast `/Game/ViS/Blueprint/GameState/GS_ViS` (`GameplayStatics.GetGameState`)))
  (`KismetArrayLibrary.Array_Add` (`/Game/ViS/Blueprint/GameState/GS_ViS.Artefacts` _asgs_vi_s) self))