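; Player controller that shows a lobby UI on start and switches the player into gameplay controls when the match begins.
; BeginPlay creates the WG_Lobby widget once, caches it, adds it to the viewport and shows the mouse cursor.
; OnMatchStart removes the lobby widget, hides the cursor and adds the IMC_Movement Enhanced Input mapping context, so movement input is only mapped after the match starts.
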(event `self.ReceiveBeginPlay`
  (`self.DisplayLobbyUI`))

(event `OnMatchStart`
  (`self.HideLobbyUI`)
  (`EnhancedInputSubsystemInterface.AddMappingContext` (pcsubsystem `EnhancedInputLocalPlayerSubsystem` self) "/Game/ViUe/Input/IMC_Movement.IMC_Movement" 0 (struct)))

(fn `DisplayLobbyUI`
  (`/Engine/EditorBlueprintResources/StandardMacros.IsValid` (`self.LobbyUI`)
    (:`Is Valid`
      _)
    (:`Is Not Valid`
      (bind _returnvalue (`|CreateWidget` "/Game/ViUe/UI/Menu/WG_Lobby.WG_Lobby_C" self))
      (set `self.LobbyUI` _returnvalue)))
  (`UserWidget.AddToViewport` (`self.LobbyUI`) 0)
  (set `self.bShowMouseCursor` true))

(fn `HideLobbyUI`
  (`Widget.RemoveFromParent` (`self.LobbyUI`))
  (set `self.bShowMouseCursor` false))

(fn `UserConstructionScript`)