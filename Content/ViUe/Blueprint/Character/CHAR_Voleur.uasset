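; CHAR_Voleur is the thief character Blueprint, which tracks whether the thief is inside the map.
; EnterMap and LeaveMap set the VoleurState enum, and IsInside reports whether it holds the entered state.
; Each transition also switches the EntranceExitBound collision object type between two custom channels and prints a French message announcing the entry or exit.
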(fn `EnterMap`
  (set `self.VoleurState` "NewEnumerator1")
  (`PrimitiveComponent.SetCollisionObjectType` (`self.EntranceExitBound`) "ECC_GameTraceChannel2")
  (`KismetSystemLibrary.PrintString` "Vous entrez dans la carte"))

(fn `IsInside`
  (returns (IsInside :type Boolean))
  (return (`|EnumEquality` (`self.VoleurState`) "NewEnumerator1")))

(fn `LeaveMap`
  (set `self.VoleurState` "NewEnumerator2")
  (`PrimitiveComponent.SetCollisionObjectType` (`self.EntranceExitBound`) "ECC_GameTraceChannel1")
  (`KismetSystemLibrary.PrintString` "Vous quittez la carte"))

(fn `UserConstructionScript`)