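; Main menu player controller that opens the WG_MainMenu widget on BeginPlay and shows the mouse cursor.
; GoToWidget runs only on the local controller, removing the open menu and displaying the requested widget class as the new OpenedMenu.
; It reuses a widget found in the CachedMenus map or creates one otherwise, though this file never adds created widgets to that map.
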(event `self.ReceiveBeginPlay`
  (`self.GoToWidget` "/Game/ViUe/UI/Menu/WG_MainMenu.WG_MainMenu_C")
  (set `self.bShowMouseCursor` true))

(fn `GoToWidget`
  (params (WidgetClass :type "UserWidget Class Reference"))
  (bind _openedmenu (`self.OpenedMenu`))
  (bind (_value _returnvalue) (`BlueprintMapLibrary.Map_Find` (`self.CachedMenus`) WidgetClass))
  (if (`self.IsLocalPlayerController`)
    ;[1 1 1] Close current widget
    (`/Engine/EditorBlueprintResources/StandardMacros.IsValid` _openedmenu
      (:`Is Valid`
        (`Widget.RemoveFromParent` _openedmenu))
      (:`Is Not Valid`
        _))
    ;[1 1 1] If menu cached
    (if _returnvalue
      ;[1 1 1] Display cached menu
      (bind _output_get (set `self.OpenedMenu` _value))
      (`UserWidget.AddToViewport` _output_get 0)
      (else
        ;[1 1 1] Display created menu
        (bind _returnvalue_2 (`|CreateWidget` WidgetClass self))
        (bind _output_get_2 (set `self.OpenedMenu` _returnvalue_2))
        (`UserWidget.AddToViewport` _output_get_2 0)))))

(fn `UserConstructionScript`)